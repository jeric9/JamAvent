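; BP_CameraManager is a camera actor that follows the BP_Chara character along a spline path.
; On BeginPlay it finds and caches the character, then each Tick runs MoveCamera while that reference is valid.
; MoveCamera snaps the Camera to the spline point closest to the character's capsule position, offset along world X, without interpolation.
; An older fixed-offset move of the root component remains unconnected.
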(event Custom|MoveCamera
  (bind _chararef (Variables|Default|GetCharaRef))
  (bind _capsulecomponent (Variables|/Script/Engine.Character|GetCapsuleComponent _chararef))
  (bind _returnvalue (Transformation|GetWorldLocation _capsulecomponent))
  (Transformation|SetWorldLocation (Variables|Default|GetCamera) (Class|SplineComponent|GetLocationatSplineInputKey (Variables|Default|GetSpline) (Class|SplineComponent|FindInputKeyClosesttoWorldLocation (Variables|Default|GetSpline) (Math|Vector|MakeVector (+ (.x _returnvalue) 215.0) (.y _returnvalue) (.z _returnvalue))) "World") false false))

(event EventBeginPlay
  (bind _returnvalue (Actor|GetActorOfClass "/Game/BluePrints/BP_Chara.BP_Chara_C"))
  (bind _output_get (Variables|Default|SetCharaRef _returnvalue))
  (Variables|Default|SetisCharaOK (Utilities|IsValid _output_get)))

(event Collision|EventActorBeginOverlap
  (params (OtherActor :type Actor%20Object%20Reference)))

(event EventTick
  (params (DeltaSeconds :type Float%20%28single-precision%29))
  (if (Variables|Default|GetisCharaOK)
    (CallFunction|MoveCamera)))

(fn ConstructionScript)
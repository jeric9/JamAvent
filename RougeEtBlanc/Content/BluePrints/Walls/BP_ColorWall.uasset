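; BP_ColorWall is a two-colour wall that costs the player character HP when touched in the wrong colour.
; The construction script applies a white or red material to the cube from the IsWhite flag.
; When BP_Chara overlaps the box with a different IsWhite value, the wall calls its LoseHP.
; The wall also binds the R key to reload Game_Lvl.
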(event OnComponentBeginOverlap(Box)
  (params (OverlappedComponent :type Primitive%20Component%20Object%20Reference) (OtherActor :type Actor%20Object%20Reference) (OtherComp :type Primitive%20Component%20Object%20Reference) (OtherBodyIndex :type Integer) (bFromSweep :type Boolean) (SweepResult :type Hit%20Result%20Structure%20%28by%20ref%29))
  (bind _asbp_chara (Utilities|Casting|CastToBP_Chara OtherActor))
  (if (not (== (Variables|Default|GetisWhite) (Variables|/Game/BluePrints/BP_Chara.BP_Chara_C|GetisWhite _asbp_chara)))
    (Default|LoseHP _asbp_chara)))

(event EventBeginPlay)

(event Collision|EventActorBeginOverlap
  (params (OtherActor :type Actor%20Object%20Reference)))

(event EventTick
  (params (DeltaSeconds :type Float%20%28single-precision%29)))

(event Input|KeyboardEvents|R
  (params (Key :type Key%20Structure :default "None"))
  (:Pressed
    (Game|OpenLevel(byName) "Game_Lvl")))

(fn ConstructionScript
  (if (Variables|Default|GetisWhite)
    (Rendering|Material|SetMaterial (Variables|Default|GetCube) 0 "/Game/Assets/Mat_Blanc.Mat_Blanc")
    (else
      (Rendering|Material|SetMaterial (Variables|Default|GetCube) 0 "/Game/Assets/Mat_Rouge.Mat_Rouge"))))
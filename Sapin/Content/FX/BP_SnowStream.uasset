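; BP_SnowStream is an effect actor that positions and orients a snowstorm effect, NSSnowStorm, on a spline.
; Each Tick places the effect at the location and rotation for SplineDistance, then adds Speed without delta-time scaling.
; The reset check zeroes SplineDistance while it is less than the spline length, so as written the effect stays at the spline start whenever the distance is below that length.
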(event EventBeginPlay)

(event Collision|EventActorBeginOverlap
  (params (OtherActor :type Actor%20Object%20Reference)))

(event EventTick
  (params (DeltaSeconds :type Float%20%28single-precision%29))
  (bind _spline (Variables|Default|GetSpline))
  (if (< (Variables|Default|GetSplineDistance) (Spline|GetSplineLength _spline))
    (Variables|Default|SetSplineDistance 0.0))
  (Transformation|SetWorldLocationAndRotation (Variables|Default|GetNS_SnowStorm) (Spline|GetLocationatDistanceAlongSpline _spline (Variables|Default|GetSplineDistance) "World") (Spline|GetRotationatDistanceAlongSpline _spline (Variables|Default|GetSplineDistance) "World") false false)
  (Variables|Default|SetSplineDistance (+ (Variables|Default|GetSplineDistance) (Variables|Default|GetSpeed))))

(fn ConstructionScript)
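; BP_ColorWall is a wall obstacle that is either white or red and damages a player character of the opposite color.
; Its construction script sets four sprites to the white or red square from the IsWhite flag.
; When BP_Chara overlaps the Box, the wall compares both IsWhite flags and calls LoseHP on a mismatch.
; It also binds the R key to reload Game_Lvl.
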(event OnComponentBeginOverlap(Box)
  (params (OverlappedComponent :type Primitive%20Component%20Object%20Reference) (OtherActor :type Actor%20Object%20Reference) (OtherComp :type Primitive%20Component%20Object%20Reference) (OtherBodyIndex :type Integer) (bFromSweep :type Boolean) (SweepResult :type Hit%20Result%20Structure%20%28by%20ref%29))
  (bind _asbp_chara (Utilities|Casting|CastToBP_Chara OtherActor))
  (if (not (== (Variables|Default|GetisWhite) (Variables|/Game/BluePrints/BP_Chara.BP_Chara_C|GetisWhite _asbp_chara)))
    (Default|LoseHP _asbp_chara)))

(event EventBeginPlay)

(event Collision|EventActorBeginOverlap
  (params (OtherActor :type Actor%20Object%20Reference)))

(event EventTick
  (params (DeltaSeconds :type Float%20%28single-precision%29)))

(event Input|KeyboardEvents|R
  (params (Key :type Key%20Structure :default "None"))
  (:Pressed
    (Game|OpenLevel(byName) "Game_Lvl")))

(fn ConstructionScript
  (bind _care_roucge_sprite (Variables|Default|Getcare_roucge_Sprite))
  (bind _care_roucge_sprite1 (Variables|Default|Getcare_roucge_Sprite1))
  (bind _care_roucge_sprite2 (Variables|Default|Getcare_roucge_Sprite2))
  (bind _care_roucge_sprite3 (Variables|Default|Getcare_roucge_Sprite3))
  (if (Variables|Default|GetisWhite)
    (Rendering|Components|Sprite|SetSprite _care_roucge_sprite "/Game/Assets/SpriteFactory/caree_blanc_Sprite.caree_blanc_Sprite")
    (Rendering|Components|Sprite|SetSprite _care_roucge_sprite1 "/Game/Assets/SpriteFactory/caree_blanc_Sprite.caree_blanc_Sprite")
    (Rendering|Components|Sprite|SetSprite _care_roucge_sprite2 "/Game/Assets/SpriteFactory/caree_blanc_Sprite.caree_blanc_Sprite")
    (Rendering|Components|Sprite|SetSprite _care_roucge_sprite3 "/Game/Assets/SpriteFactory/caree_blanc_Sprite.caree_blanc_Sprite")
    (else
      (Rendering|Components|Sprite|SetSprite _care_roucge_sprite "/Game/Assets/SpriteFactory/care_roucge_Sprite.care_roucge_Sprite")
      (Rendering|Components|Sprite|SetSprite _care_roucge_sprite1 "/Game/Assets/SpriteFactory/care_roucge_Sprite.care_roucge_Sprite")
      (Rendering|Components|Sprite|SetSprite _care_roucge_sprite2 "/Game/Assets/SpriteFactory/care_roucge_Sprite.care_roucge_Sprite")
      (Rendering|Components|Sprite|SetSprite _care_roucge_sprite3 "/Game/Assets/SpriteFactory/care_roucge_Sprite.care_roucge_Sprite"))))
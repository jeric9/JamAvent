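; BP_Key is a key pickup that unlocks its matching door when the player character touches it.
; On box overlap with BP_Chara it prints "Got Key" and searches all BP_Door actors for the first whose DoorRef equals its own.
; It calls OpenDoor on that door and destroys itself only if a match was opened.
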(event OnComponentBeginOverlap(Box)
  (params (OverlappedComponent :type Primitive%20Component%20Object%20Reference) (OtherActor :type Actor%20Object%20Reference) (OtherComp :type Primitive%20Component%20Object%20Reference) (OtherBodyIndex :type Integer) (bFromSweep :type Boolean) (SweepResult :type Hit%20Result%20Structure%20%28by%20ref%29))
  (Utilities|Casting|CastToBP_Chara OtherActor)
  (Development|PrintString "Got Key")
  (bind _outactors (Actor|GetAllActorsOfClass "/Game/BluePrints/Door/BP_Door.BP_Door_C"))
  (bind _array_element (Utilities|Array|ForEachLoopwithBreak _outactors :!label _label)
    (:LoopBody
      (if (Utilities|Enum|Equal(Enum) (Variables|/Game/BluePrints/Door/BP_Door.BP_Door_C|GetDoorRef _array_element) (Variables|Default|GetDoorRef))
        (Default|OpenDoor _array_element)
        (Variables|Default|SethasOpen true)
        (goto _label Break)))
    (:Completed
      (if (Variables|Default|GethasOpen)
        (Actor|DestroyActor)))))

(event EventBeginPlay)

(event EventTick
  (params (DeltaSeconds :type Float%20%28single-precision%29)))

(fn ConstructionScript)
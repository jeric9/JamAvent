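; BP_Destructible_Wall is a wall that is destroyed, along with the projectile, when a BP_Bullet overlaps its Box.
; When a falling third-person character overlaps the Box, it triggers a camera shake through a DoOnce that resets after a short delay.
; It also sets the character's IsAgainstWall flag and starts its LoopIsAgainstWallVelocity routine if not already looping, clearing the flag on end overlap.
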(event OnComponentBeginOverlap(Box)
  (params (OverlappedComponent :type Primitive%20Component%20Object%20Reference) (OtherActor :type Actor%20Object%20Reference) (OtherComp :type Primitive%20Component%20Object%20Reference) (OtherBodyIndex :type Integer) (bFromSweep :type Boolean) (SweepResult :type Hit%20Result%20Structure%20%28by%20ref%29))
  (bind _asbp_third_person_character (Utilities|Casting|CastToBP_ThirdPersonCharacter OtherActor)
    (:then
      (if (AI|Components|NavMovement|IsFalling (Variables|/Script/Engine.Character|GetCharacterMovement _asbp_third_person_character))
        (Utilities|FlowControl|Sequence
          (:then_0
            (Utilities|FlowControl|DoOnce false :!label _label
              (:Completed
                (Default|CameraShake _asbp_third_person_character))))
          (:then_1
            (Utilities|FlowControl|Delay 0.2)
            (goto _label Reset))))
      (if (and (AI|Components|NavMovement|IsFalling (Variables|/Script/Engine.Character|GetCharacterMovement _asbp_third_person_character)) (== (Variables|/Game/ThirdPerson/Blueprints/BP_ThirdPersonCharacter.BP_ThirdPersonCharacter_C|GetisLoopAgainstWall _asbp_third_person_character) false))
        (Variables|/Game/ThirdPerson/Blueprints/BP_ThirdPersonCharacter.BP_ThirdPersonCharacter_C|SetisAgainstWall _asbp_third_person_character true)
        (Default|LoopIsAgainstWallVelocity _asbp_third_person_character)))
    (:CastFailed
      (bind _asbp_bullet (Utilities|Casting|CastToBP_Bullet OtherActor))
      (Utilities|IsValid _asbp_bullet
        (:Is%20Valid
          (Actor|DestroyActor _asbp_bullet)
          (Actor|DestroyActor))))))

(event OnComponentEndOverlap(Box)
  (params (OverlappedComponent :type Primitive%20Component%20Object%20Reference) (OtherActor :type Actor%20Object%20Reference) (OtherComp :type Primitive%20Component%20Object%20Reference) (OtherBodyIndex :type Integer))
  (bind _asbp_third_person_character (Utilities|Casting|CastToBP_ThirdPersonCharacter OtherActor))
  (Variables|/Game/ThirdPerson/Blueprints/BP_ThirdPersonCharacter.BP_ThirdPersonCharacter_C|SetisAgainstWall _asbp_third_person_character false))

(event EventBeginPlay)

(event Collision|EventActorBeginOverlap
  (params (OtherActor :type Actor%20Object%20Reference)))

(event EventTick
  (params (DeltaSeconds :type Float%20%28single-precision%29)))

(fn ConstructionScript)
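; Bullet projectile for the player's abilities, fired either along X by a signed direction or straight up along Z.
; Shot and UpShot each fire once, starting their own timeline and a one-second self-destruct delay.
; Each timeline update applies a swept world offset scaled by the curve and bullet speed, with no hit or damage handling here.
; Shot also prints its direction for debugging.
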(event Custom|ExistenceTimeManage
  (bind _self self)
  (Utilities|FlowControl|Delay 1.0)
  (Utilities|IsValid _self
    (:Is%20Valid
      (Actor|DestroyActor _self))))

(event Custom|Shot
  (params (AnchorLocation :type Vector) (ShotDirection :type Float%20%28double-precision%29))
  (Utilities|FlowControl|DoOnce false
    (:Completed
      (Development|PrintString (Utilities|String|Append "FORWARD X ANCHOR SHOOT POINT" (Utilities|String|ToString(Float) ShotDirection)))
      (CallFunction|ExistenceTimeManage)
      (bind _t_bulletshotpercentdist (Timeline|Timeline PlayFromStart)
        (:Update
          (Transformation|AddActorWorldOffset (Math|Vector|MakeVector (* _t_bulletshotpercentdist (* (Variables|Default|GetBULLET_SPEED) 3.0) ShotDirection) 0.0 0.0) true))))))

(event Custom|UpShot
  (Utilities|FlowControl|DoOnce false
    (:Completed
      (CallFunction|ExistenceTimeManage)
      (bind _t_bulletshotpercentdist (Timeline|Timeline_0 PlayFromStart)
        (:Update
          (Transformation|AddActorWorldOffset (Math|Vector|MakeVector 0.0 0.0 (* _t_bulletshotpercentdist (* (Variables|Default|GetBULLET_SPEED) 3.0))) true))))))

(event EventBeginPlay)

(event Collision|EventActorBeginOverlap
  (params (OtherActor :type Actor%20Object%20Reference)))

(event EventTick
  (params (DeltaSeconds :type Float%20%28single-precision%29)))

(fn ConstructionScript)
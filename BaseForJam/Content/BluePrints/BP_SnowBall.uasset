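; BP_SnowBall is a snowball actor whose sphere rolls back and forth along a spline in an endless loop.
; On BeginPlay it starts the movement, first waiting briefly when IsSync is false so it runs out of phase.
; A slowed timeline drives the spline input key for the sphere's relative location, and a FlipFlop on Finished alternates reverse and forward playback.
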(event Custom|LoopRollSpline
  (Components|Timeline|SetPlayRate (Variables|Default|GetTL_RollSpline) 0.25)
  (bind _t_upanddownslpine (Timeline|TL_RollSpline PlayFromStart)
    (:Update
      (Transformation|SetRelativeLocation (Variables|Default|GetSphere) (Class|SplineComponent|GetLocationatSplineInputKey (Variables|Default|GetSpline) _t_upanddownslpine "Local") false false))
    (:Finished
      (Utilities|FlowControl|FlipFlop
        (:A
          (Timeline|TL_RollSpline ReverseFromEnd))
        (:B
          (Timeline|TL_RollSpline PlayFromStart))))))

(event EventBeginPlay
  (if (Variables|Default|GetisSync)
    _
    (else
      (Utilities|FlowControl|Delay 1.5)))
  (CallFunction|LoopRollSpline))

(event Collision|EventActorBeginOverlap
  (params (OtherActor :type Actor%20Object%20Reference)))

(event EventTick
  (params (DeltaSeconds :type Float%20%28single-precision%29)))

(fn ConstructionScript)
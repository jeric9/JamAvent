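; BP_StormManager is a manager Blueprint that triggers a storm effect for player 1 or player 2.
; On BeginPlay it finds the BP_Storm actors and caches those whose StormRef is "storm1" or "storm2".
; The callstorm event takes a player index and activates that storm's NSStorm component.
; It prints start and end messages around a STORMDURATION delay, but never deactivates the effect itself.
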(event Custom|call%20storm
  (params (index :type Integer))
  (bind _storm_duration (Variables|Default|GetSTORM_DURATION))
  ;[1 1 1] index = 1 ou 2 selon joueur 1 ou 2
  (if (== index 1)
    (Components|Activation|Activate (Variables|/Game/BluePrints/Storm/BP_Storm.BP_Storm_C|GetNS_Storm (Variables|Default|GetBP_StormRef_1)) false)
    (Development|PrintString "THE STORM FOR PLAYER 1 !!!!")
    (Utilities|FlowControl|Delay _storm_duration)
    (Development|PrintString "END STORM FOR PLAYER 1 !!!!")
    (elif (== index 2)
      (Components|Activation|Activate (Variables|/Game/BluePrints/Storm/BP_Storm.BP_Storm_C|GetNS_Storm (Variables|Default|GetBP_StormRef_2)) false)
      (Development|PrintString "THE STORM FOR PLAYER 2 !!!!")
      (Utilities|FlowControl|Delay _storm_duration)
      (Development|PrintString "END STORM FOR PLAYER 2 !!!!"))))

(event EventBeginPlay
  (bind _outactors (Actor|GetAllActorsOfClass "/Game/BluePrints/Storm/BP_Storm.BP_Storm_C"))
  (for _array_element _outactors
    (if (Utilities|Enum|Equal(Enum) (Variables|/Game/BluePrints/Storm/BP_Storm.BP_Storm_C|GetStormRef _array_element) "storm1")
      (Variables|Default|SetBP_StormRef_1 _array_element)
      (elif (Utilities|Enum|Equal(Enum) (Variables|/Game/BluePrints/Storm/BP_Storm.BP_Storm_C|GetStormRef _array_element) "storm2")
        (Variables|Default|SetBP_StormRef_2 _array_element)))))

(event Collision|EventActorBeginOverlap
  (params (OtherActor :type Actor%20Object%20Reference)))

(event EventTick
  (params (DeltaSeconds :type Float%20%28single-precision%29)))

(fn ConstructionScript)
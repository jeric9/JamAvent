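; BP_Mage is an actor that endlessly moves its Cube component along its Spline, apparently a circular path.
; On BeginPlay, a slowed timeline starts and restarts itself whenever it finishes.
; Each update scales the timeline value into a spline input key, rather than a distance, and sets the cube's relative location from that point in local space.
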(event Custom|LoopCircleAlongSpline
  (Components|Timeline|SetPlayRate (Variables|Default|GetTL_LoopCircle) 0.25)
  (bind _t_loopcirclespline (Timeline|TL_LoopCircle PlayFromStart)
    (:Update
      (Transformation|SetRelativeLocation (Variables|Default|GetCube) (Class|SplineComponent|GetLocationatSplineInputKey (Variables|Default|GetSpline) (* _t_loopcirclespline 4.0) "Local") false false))
    (:Finished
      (Timeline|TL_LoopCircle PlayFromStart))))

(event EventBeginPlay
  (CallFunction|LoopCircleAlongSpline))

(event Collision|EventActorBeginOverlap
  (params (OtherActor :type Actor%20Object%20Reference)))

(event EventTick
  (params (DeltaSeconds :type Float%20%28single-precision%29)))

(fn ConstructionScript)
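; BP_Stalag is an actor that moves its static mesh back and forth along a spline in an endless loop.
; On BeginPlay it starts a slowed timeline, after a short delay unless IsSync is set, which offsets unsynced instances.
; The timeline drives the spline input key for the mesh location, and a FlipFlop on finish alternates reverse and forward playback.
; The construction script places a preview mesh at spline key 1.
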(event Custom|LoopUpAndDown
  (Components|Timeline|SetPlayRate (Variables|Default|GetTL_UpAndDownSlide) 0.25)
  (bind _t_upanddownslpine (Timeline|TL_UpAndDownSlide PlayFromStart)
    (:Update
      (Transformation|SetRelativeLocation (Variables|Default|GetStaticMesh) (Class|SplineComponent|GetLocationatSplineInputKey (Variables|Default|GetSpline) _t_upanddownslpine "Local") false false))
    (:Finished
      (Utilities|FlowControl|FlipFlop
        (:A
          (Timeline|TL_UpAndDownSlide ReverseFromEnd))
        (:B
          (Timeline|TL_UpAndDownSlide PlayFromStart))))))

(event EventBeginPlay
  (if (Variables|Default|GetisSync)
    _
    (else
      (Utilities|FlowControl|Delay 1.5)))
  (CallFunction|LoopUpandDown))

(event Collision|EventActorBeginOverlap
  (params (OtherActor :type Actor%20Object%20Reference)))

(event EventTick
  (params (DeltaSeconds :type Float%20%28single-precision%29)))

(fn ConstructionScript
  (Transformation|SetRelativeLocation (Variables|Default|GetStaticMeshPreview) (Class|SplineComponent|GetLocationatSplineInputKey (Variables|Default|GetSpline) 1.0 "Local") false false))
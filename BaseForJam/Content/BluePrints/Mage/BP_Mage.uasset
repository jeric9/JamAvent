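; BP_Mage is a mage actor that summons a storm through BP_StormManager unless a character stops it first.
; A timeline endlessly moves its Cube along a spline.
; The first capsule overlap plays a voice and, for a player character, starts a delay before calling CallStorm with the other player's index.
; A character hitting the Cube destroys the mage and cancels the storm; the Zgrub countdown helper is never called here.
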(event OnComponentBeginOverlap(DetectCapsule)
  (params (OverlappedComponent :type Primitive%20Component%20Object%20Reference) (OtherActor :type Actor%20Object%20Reference) (OtherComp :type Primitive%20Component%20Object%20Reference) (OtherBodyIndex :type Integer) (bFromSweep :type Boolean) (SweepResult :type Hit%20Result%20Structure%20%28by%20ref%29))
  (bind _gi_ref (Variables|Default|GetGI_Ref))
  (bind _before_storm_duration (Variables|Default|GetBEFORE_STORM_DURATION))
  (Utilities|FlowControl|DoOnce false
    (:Completed
      (bind _asbp_chara (Utilities|Casting|CastToBP_Chara OtherActor))
      (Audio|PlaySoundatLocation "/Game/Audio/voix/voix.voix" (Transformation|GetWorldLocation (Variables|Default|GetCube)) "0, 0, 0" 1.0 1.0 0.0 0 0 0 0)
      (if (== _asbp_chara (Variables|/Game/GI_Base.GI_Base_C|Getchara1 _gi_ref))
        (Development|PrintString "start timer before storm for 1")
        (Variables|Default|Setindex 2)
        (Variables|Default|SetBeforeStormTime _before_storm_duration :!label _label)
        (Utilities|FlowControl|Delay _before_storm_duration)
        (if (Variables|Default|GetisCanCallStorm)
          (Default|CallStorm (Variables|Default|GetBP_StormManagerRef) (Variables|Default|Getindex)))
        (elif (== _asbp_chara (Variables|/Game/GI_Base.GI_Base_C|Getchara2 _gi_ref))
          (Development|PrintString "start timer before storm for 2")
          (Variables|Default|Setindex 1)
          (goto _label))))))

(event OnComponentHit(Cube)
  (params (HitComponent :type Primitive%20Component%20Object%20Reference) (OtherActor :type Actor%20Object%20Reference) (OtherComp :type Primitive%20Component%20Object%20Reference) (NormalImpulse :type Vector :default "0, 0, 0") (Hit :type Hit%20Result%20Structure%20%28by%20ref%29))
  (Utilities|Casting|CastToBP_Chara OtherActor)
  (Variables|Default|SetisCanCallStorm false)
  (Actor|DestroyActor))

(event Custom|LoopCircleAlongSpline
  (Components|Timeline|SetPlayRate (Variables|Default|GetTL_LoopCircle) 0.25)
  (bind _t_loopcirclespline (Timeline|TL_LoopCircle PlayFromStart)
    (:Update
      (Transformation|SetRelativeLocation (Variables|Default|GetCube) (Class|SplineComponent|GetLocationatSplineInputKey (Variables|Default|GetSpline) (* _t_loopcirclespline 4.0) "Local") false false))
    (:Finished
      (Timeline|TL_LoopCircle PlayFromStart))))

(event Custom|ForceStopTimerBeforeStorm
  (Utilities|Time|ClearTimerbyFunctionName 0 "TimerBeforeStorm"))

(event EventBeginPlay
  (bind _asgi_base (Utilities|Casting|CastToGI_Base (Game|GetGameInstance)))
  (Variables|Default|SetGI_Ref _asgi_base)
  (bind _returnvalue (Actor|GetActorOfClass "/Game/BluePrints/Storm/BP_StormManager.BP_StormManager_C"))
  (Variables|Default|SetBP_StormManagerRef _returnvalue)
  (CallFunction|LoopCircleAlongSpline))

(event Collision|EventActorBeginOverlap
  (params (OtherActor :type Actor%20Object%20Reference)))

(event EventTick
  (params (DeltaSeconds :type Float%20%28single-precision%29)))

(fn ConstructionScript)

(fn Zgrub
  (params (NewParam :type Boolean))
  ;[1 1 1] Decrement -1 milliseconds if not 0 or inf. ELSE Force STOP FreezeByIceTimer
  (if (<= (Variables|Default|GetBeforeStormTime) 0.0)
    (CallFunction|ForceStopTimerBeforeStorm)
    (else
      (bind _result (Math|Float|DecrementFloat (Variables|Default|GetBeforeStormTime))
        (:%20%20
          (Variables|Default|SetBeforeStormTime _result))))))
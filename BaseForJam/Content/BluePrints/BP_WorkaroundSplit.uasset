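; Debug-style workaround actor, apparently for split-screen, that hands a tagged character to the second player.
; The gamepad bottom face button finds actors tagged "2", casts them to BP_Chara and has player controller ID 1 possess them, printing debug messages.
; A matching branch for tag "1" and player controller 0 is unwired, and Tick only reaches an empty DoOnce.
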(event EventBeginPlay)

(event Collision|EventActorBeginOverlap
  (params (OtherActor :type Actor%20Object%20Reference)))

(event EventTick
  (params (DeltaSeconds :type Float%20%28single-precision%29))
  (if true
    (Utilities|FlowControl|DoOnce false)))

(event Input|GamepadEvents|GamepadFaceButtonBottom
  (params (Key :type Key%20Structure :default "None"))
  (bind _returnvalue (Class|GameplayStatics|GetPlayerControllerfromID 1))
  (:Pressed
    (Development|PrintString "face btn bottom vanilla")
    (bind _outactors (Actor|GetAllActorswithTag "2"))
    (for _array_element _outactors
      (bind _asbp_chara (Utilities|Casting|CastToBP_Chara _array_element))
      (Utilities|IsValid _returnvalue
        (:Is%20Valid
          (Pawn|Possess _returnvalue _asbp_chara))
        (:Is%20Not%20Valid
          (Development|PrintString "GET PLAYER CONTROLLER NOT FOUND"))))))

(event Input|KeyboardEvents|Enter
  (params (Key :type Key%20Structure :default "None")))

(fn ConstructionScript)
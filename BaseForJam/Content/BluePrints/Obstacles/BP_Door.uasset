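; BP_Door is an obstacle door that slides its static mesh along a spline when its OpenTheDoor event fires.
; OpenTheDoor plays a snow-rolling sound at the mesh, then runs a timeline whose track drives the spline input key, setting the mesh's world location without sweep.
; The construction script snaps Cube1 to the spline point at key 1, apparently marking the open position in the editor.
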(event Custom|OpenTheDoor
  (bind _staticmesh (Variables|Default|GetStaticMesh))
  (Audio|PlaySoundatLocation "/Game/Audio/roullement_de_neige.roullement_de_neige" (Transformation|GetWorldLocation _staticmesh) "0, 0, 0" 1.0 1.0 0.0 0 0 0 0)
  (bind _newtrack_0 (Timeline|TL_OpenDoor PlayFromStart)
    (:Update
      (Transformation|SetWorldLocation _staticmesh (Class|SplineComponent|GetLocationatSplineInputKey (Variables|Default|GetSpline) _newtrack_0 "World") false false))))

(event EventBeginPlay)

(event Collision|EventActorBeginOverlap
  (params (OtherActor :type Actor%20Object%20Reference)))

(event EventTick
  (params (DeltaSeconds :type Float%20%28single-precision%29)))

(fn ConstructionScript
  (Transformation|SetRelativeLocation (Variables|Default|GetCube1) (Class|SplineComponent|GetLocationatSplineInputKey (Variables|Default|GetSpline) 1.0 "Local") false false))
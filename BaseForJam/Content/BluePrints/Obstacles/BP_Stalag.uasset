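; BP_Stalag is a moving obstacle that opens Game_Lvl when its mesh hits BP_Chara.
; A slowed timeline slides the mesh along a local spline, with a FlipFlop on Finished alternating reverse and forward play to loop endlessly.
; Movement starts on BeginPlay, delayed briefly when IsSync is false to offset instances.
; The construction script places a preview mesh at spline key 1 to show the travel target.
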(event OnComponentHit(StaticMesh)
  (params (HitComponent :type Primitive%20Component%20Object%20Reference) (OtherActor :type Actor%20Object%20Reference) (OtherComp :type Primitive%20Component%20Object%20Reference) (NormalImpulse :type Vector :default "0, 0, 0") (Hit :type Hit%20Result%20Structure%20%28by%20ref%29))
  (Utilities|Casting|CastToBP_Chara OtherActor)
  (Game|OpenLevel(byName) "Game_Lvl"))

(event Custom|LoopUpAndDown
  (Components|Timeline|SetPlayRate (Variables|Default|GetTL_UpAndDownSlide) 0.25)
  (bind _t_upanddownslpine (Timeline|TL_UpAndDownSlide PlayFromStart)
    (:Update
      (Transformation|SetRelativeLocation (Variables|Default|GetStaticMesh) (Class|SplineComponent|GetLocationatSplineInputKey (Variables|Default|GetSpline) _t_upanddownslpine "Local") false false))
    (:Finished
      (Utilities|FlowControl|FlipFlop
        (:A
          (Timeline|TL_UpAndDownSlide ReverseFromEnd))
        (:B
          (Timeline|TL_UpAndDownSlide PlayFromStart))))))

(event EventBeginPlay
  (if (Variables|Default|GetisSync)
    _
    (else
      (Utilities|FlowControl|Delay 1.5)))
  (CallFunction|LoopUpandDown))

(event Collision|EventActorBeginOverlap
  (params (OtherActor :type Actor%20Object%20Reference)))

(event EventTick
  (params (DeltaSeconds :type Float%20%28single-precision%29)))

(fn ConstructionScript
  (Transformation|SetRelativeLocation (Variables|Default|GetStaticMeshPreview) (Class|SplineComponent|GetLocationatSplineInputKey (Variables|Default|GetSpline) 1.0 "Local") false false))